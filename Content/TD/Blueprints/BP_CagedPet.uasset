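; BP_CagedPet is a caged pet actor that a player character can release.
; Its Trigger overlap events set the player's CurrentCage to this actor on entry and clear it on exit.
; FreePet destroys only the Cage component, then spawns a BP_Pet and assigns the passed Owner as its OwningPlayer.
; Nothing in this Blueprint calls FreePet itself.
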(event `self.Trigger.OnComponentBeginOverlap`
  (params (OverlappedComponent :type "PrimitiveComponent Object Reference") (OtherActor :type "Actor Object Reference") (OtherComp :type "PrimitiveComponent Object Reference") (OtherBodyIndex :type Integer) (bFromSweep :type Boolean) (SweepResult :type "HitResult Structure (by ref)"))
  (bind _asbp_player_character (cast `/Game/TD/Blueprints/Player/BP_PlayerCharacter` OtherActor))
  (set `/Game/TD/Blueprints/Player/BP_PlayerCharacter.CurrentCage` self _asbp_player_character))

(event `self.Trigger.OnComponentEndOverlap`
  (params (OverlappedComponent :type "PrimitiveComponent Object Reference") (OtherActor :type "Actor Object Reference") (OtherComp :type "PrimitiveComponent Object Reference") (OtherBodyIndex :type Integer))
  (bind _asbp_player_character (cast `/Game/TD/Blueprints/Player/BP_PlayerCharacter` OtherActor))
  (set `/Game/TD/Blueprints/Player/BP_PlayerCharacter.CurrentCage` null _asbp_player_character))

(fn `Free Pet`
  (params (Owner :type "/Game/TD/Blueprints/Player/BP_PlayerCharacter Object Reference"))
  (`ActorComponent.K2_DestroyComponent` (`self.Cage`))
  (bind _returnvalue (`|SpawnActorFromClass` "/Game/TD/Blueprints/BP_Pet.BP_Pet_C" (`KismetMathLibrary.MakeTransform` (0.0 0.0 0.0)) "Undefined" "MultiplyWithRoot" null null))
  (set `/Game/TD/Blueprints/BP_Pet.OwningPlayer` Owner _returnvalue))

(fn `UserConstructionScript`)