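; Interactable factory core that starts a timed self-destruct of an enemy camp.
; A sphere overlap registers the core on the player pet; Interact then shows a countdown widget, enables the pet's door use and plays a timeline scaled to TimeToExplosion.
; The timeline drives the timer display, and EndCountdown removes the widget, destroys the factory entrance, exit and core, and prints a victory message.
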(event `self.ReceiveBeginPlay`
  (`TimelineComponent.SetPlayRate` (`self.ExplosionTimeline`) (/ 1.0 (`self.TimeToExplosion`)))
  (set `/Game/TD/Blueprints/BP_FactoryInsideVent.FactoryCore` self (`self.FactoryExit`)))

(event `self.Sphere.OnComponentBeginOverlap`
  (params (OverlappedComponent :type "PrimitiveComponent Object Reference") (OtherActor :type "Actor Object Reference") (OtherComp :type "PrimitiveComponent Object Reference") (OtherBodyIndex :type Integer) (bFromSweep :type Boolean) (SweepResult :type "HitResult Structure (by ref)"))
  (bind _asbp_player_pet (cast `/Game/TD/Blueprints/Player/BP_PlayerPet` OtherActor))
  (set `self.Player Pet` _asbp_player_pet)
  (set `/Game/TD/Blueprints/Player/BP_PlayerPet.CurrentFactoryCore` self _asbp_player_pet))

(event `self.Sphere.OnComponentEndOverlap`
  (params (OverlappedComponent :type "PrimitiveComponent Object Reference") (OtherActor :type "Actor Object Reference") (OtherComp :type "PrimitiveComponent Object Reference") (OtherBodyIndex :type Integer))
  (bind _asbp_player_pet (cast `/Game/TD/Blueprints/Player/BP_PlayerPet` OtherActor))
  (set `self.Player Pet` null)
  (set `/Game/TD/Blueprints/Player/BP_PlayerPet.CurrentFactoryCore` null _asbp_player_pet))

(fn `EndCountdown`
  (`TimelineComponent.Stop` (`self.ExplosionTimeline`))
  (`Widget.RemoveFromParent` (`self.CountDownUI`))
  (`self.K2_DestroyActor` (`self.FactoryExit`))
  (`self.K2_DestroyActor` (`self.FactoryEntrance`))
  (`KismetSystemLibrary.PrintString` "Congratulations, you destroyed the camp !" true true (struct :`G` 0.66 :`B` 1.0 :`A` 1.0) 20.0)
  (`self.K2_DestroyActor`))

(fn `Interact`
  (if (`self.IsTimeRunning`)
    (`KismetSystemLibrary.PrintString` "RUN")
    (else
      (bind _returnvalue (`|CreateWidget` "/Game/TD/Blueprints/UI/WBP_ExplosionCountDown.WBP_ExplosionCountDown_C"))
      (bind _output_get (set `self.CountDownUI` _returnvalue))
      (`UserWidget.AddToViewport` _output_get 0)
      (set `/Game/TD/Blueprints/Player/BP_PlayerPet.CanUseDoor` true (`self.Player Pet`))
      (`TimelineComponent.PlayFromStart` (`self.ExplosionTimeline`))
      (set `self.IsTimeRunning` true))))

(fn `UserConstructionScript`)