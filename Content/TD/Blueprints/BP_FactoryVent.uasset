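; BP_FactoryVent is an interactable vent where the player deploys and takes control of a robot pet.
; Its box overlap registers or clears the vent as the player character's current vent.
; Interact swaps control to the vent's existing pet through the player controller.
; Without one, it spends an available pet to spawn one at the spawn point, links it to the player and swaps, or prints a message when none remain.
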(event `self.ReceiveBeginPlay`
  (bind _returnvalue (`GameplayStatics.GetActorOfClass` "/Game/TD/Blueprints/Player/BP_PlayerCharacter.BP_PlayerCharacter_C"))
  (set `self.Player Character` _returnvalue))

(event `self.Box.OnComponentBeginOverlap`
  (params (OverlappedComponent :type "PrimitiveComponent Object Reference") (OtherActor :type "Actor Object Reference") (OtherComp :type "PrimitiveComponent Object Reference") (OtherBodyIndex :type Integer) (bFromSweep :type Boolean) (SweepResult :type "HitResult Structure (by ref)"))
  ; Send Info to player character
  (bind _asbp_player_character (cast `/Game/TD/Blueprints/Player/BP_PlayerCharacter` OtherActor))
  (bind _output_get (set `self.Player Character` _asbp_player_character))
  (set `/Game/TD/Blueprints/Player/BP_PlayerCharacter.CurrentFactoryVent` self _output_get))

(event `self.Box.OnComponentEndOverlap`
  (params (OverlappedComponent :type "PrimitiveComponent Object Reference") (OtherActor :type "Actor Object Reference") (OtherComp :type "PrimitiveComponent Object Reference") (OtherBodyIndex :type Integer))
  ; Send Info to player character
  (bind _asbp_player_character (cast `/Game/TD/Blueprints/Player/BP_PlayerCharacter` OtherActor))
  (bind _output_get (set `self.Player Character` _asbp_player_character))
  (set `/Game/TD/Blueprints/Player/BP_PlayerCharacter.CurrentFactoryVent` null _output_get))

(fn `Interact`
  (bind _player_character (`self.Player Character`))
  (bind _playerpet (`self.PlayerPet`))
  (`/Engine/EditorBlueprintResources/StandardMacros.IsValid` (`self.PlayerPet`)
    (:`Is Valid`
      (bind _asbp_player_controller (cast `/Game/TD/Blueprints/Player/BP_PlayerController` (`GameplayStatics.GetPlayerController` 0)))
      (`/Game/TD/Blueprints/Player/BP_PlayerController.SwapCharacter` _asbp_player_controller (`self.PlayerPet`)))
    (:`Is Not Valid`
      (if (> (`/Game/TD/Blueprints/Player/BP_PlayerCharacter.NumberOfPetsAvailable` (`self.Player Character`)) 0)
        (set `/Game/TD/Blueprints/Player/BP_PlayerCharacter.NumberOfPetsAvailable` (- (`/Game/TD/Blueprints/Player/BP_PlayerCharacter.NumberOfPetsAvailable` (`self.Player Character`)) 1) (`self.Player Character`))
        (bind _returnvalue (`|SpawnActorFromClass` "/Game/TD/Blueprints/Player/BP_PlayerPet.BP_PlayerPet_C" (`KismetMathLibrary.Conv_VectorToTransform` (`SceneComponent.K2_GetComponentLocation` (`self.SpawnPoint`))) "Undefined" "MultiplyWithRoot" null null))
        (set `self.PlayerPet` _returnvalue)
        (bind _asbp_player_controller_2 (cast `/Game/TD/Blueprints/Player/BP_PlayerController` (`GameplayStatics.GetPlayerController` 0)))
        (`/Game/TD/Blueprints/Player/BP_PlayerController.SwapCharacter` _asbp_player_controller_2 _playerpet)
        (set `/Game/TD/Blueprints/Player/BP_PlayerPet.PlayerCharacter` _player_character _playerpet)
        (set `/Game/TD/Blueprints/Player/BP_PlayerCharacter.CurrentPlayerPet` (`self.PlayerPet`) _player_character)
        (else
          (`KismetSystemLibrary.PrintString` "You don't have any usable robots left !" true true (struct :`G` 0.66 :`B` 1.0 :`A` 1.0) 5.0))))))

(fn `UserConstructionScript`)