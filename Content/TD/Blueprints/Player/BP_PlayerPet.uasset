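; BP_PlayerPet is the player's pet, a secondary playable character that marks itself as not the main character.
; It tracks possession and runs the parent Tick only while possessed.
; The swap input makes player controller 0 possess the stored PlayerCharacter, with debug prints for success or a missing reference.
; The interact input triggers the current factory core if valid, and any damage taken is passed to LoseHP.
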(event `self.ReceiveBeginPlay`
  (set `self.IsMainCharacter` false))

(event `self.ReceiveTick`
  (params (DeltaSeconds :type "Float (single-precision)"))
  (if (`self.IsPossessed`)
    (`parent.ReceiveTick` DeltaSeconds)))

(event `self.ReceivePossessed`
  (params (NewController :type "Controller Object Reference"))
  (set `self.IsPossessed` true))

(event `self.ReceiveUnpossessed`
  (params (OldController :type "Controller Object Reference"))
  (set `self.IsPossessed` false))

(event `EnhancedInput|/Game/TD/Input/Actions/IA_SwapCharacters`
  (params (ActionValue :type Boolean) (ElapsedSeconds :type "Float (double-precision)") (TriggeredSeconds :type "Float (double-precision)") (InputAction :type "InputAction Object Reference" :default "/Game/TD/Input/Actions/IA_SwapCharacters.IA_SwapCharacters"))
  (bind _playercharacter (`self.PlayerCharacter`))
  (:`Started`
    (`/Engine/EditorBlueprintResources/StandardMacros.IsValid` _playercharacter
      (:`Is Valid`
        (`Controller.Possess` (`GameplayStatics.GetPlayerController` 0) _playercharacter)
        (`KismetSystemLibrary.PrintString` "player character possessed"))
      (:`Is Not Valid`
        (`KismetSystemLibrary.PrintString` "no valid player character")))))

(event `EnhancedInput|/Game/TD/Input/Actions/IA_Interact`
  (params (ActionValue :type Boolean) (ElapsedSeconds :type "Float (double-precision)") (TriggeredSeconds :type "Float (double-precision)") (InputAction :type "InputAction Object Reference" :default "/Game/TD/Input/Actions/IA_Interact.IA_Interact"))
  (bind _currentfactorycore (`self.CurrentFactoryCore`))
  (:`Started`
    (`/Engine/EditorBlueprintResources/StandardMacros.IsValid` _currentfactorycore
      (:`Is Valid`
        (`/Game/TD/Blueprints/BP_FactoryCore.Interact` _currentfactorycore)))))

(event `self.ReceiveAnyDamage`
  (params (Damage :type "Float (single-precision)") (DamageType :type "DamageType Object Reference") (InstigatedBy :type "Controller Object Reference") (DamageCauser :type "Actor Object Reference"))
  (`self.LoseHP` Damage))

(fn `UserConstructionScript`
  (`parent.UserConstructionScript`))