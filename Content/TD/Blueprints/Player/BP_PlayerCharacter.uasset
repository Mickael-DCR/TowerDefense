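; Player character for a top-down game, with camera-relative movement, cursor aiming, health, and possession swapping to a pet.
; Tick turns controller yaw toward the cursor hit; primary fire spawns damage-carrying projectiles outside building mode.
; The first skill exits building mode or launches a grenade, with a timeline as its cooldown.
; Damage feeds LoseHP into Die, which casts self to BP_PlayerPet to repossess the owner and destroy the pet.
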(event `self.ReceiveBeginPlay`
  (set `PlayerController.bShowMouseCursor` true (`GameplayStatics.GetPlayerController` 0))
  (`TimelineComponent.SetPlayRate` (`self.FirstSkillCoolDown Timeline`) (/ 1.0 (`self.FirstSkillCD`))))

(event `self.ReceiveTick`
  (params (DeltaSeconds :type "Float (single-precision)"))
  (bind (_returnvalue_roll _returnvalue_pitch _returnvalue_yaw) (`KismetMathLibrary.BreakRotator` (`KismetMathLibrary.FindLookAtRotation` (`self.K2_GetActorLocation`) (`self.GetLookAtLocation`))))
  ; Makes the character look at the cursor
  (`Controller.SetControlRotation` (`GameplayStatics.GetPlayerController` 0) (`KismetMathLibrary.MakeRotator` 0.0 0.0 _returnvalue_yaw)))

(event `EnhancedInput|/Game/TD/Input/Actions/IA_Interact`
  (params (ActionValue :type Boolean) (ElapsedSeconds :type "Float (double-precision)") (TriggeredSeconds :type "Float (double-precision)") (InputAction :type "InputAction Object Reference" :default "/Game/TD/Input/Actions/IA_Interact.IA_Interact"))
  (bind _currentfactoryvent (`self.CurrentFactoryVent`))
  ; INTERACTIONS
  ;
  ; Change this logic -> interface, send messages
  (:`Triggered`
    (`/Engine/EditorBlueprintResources/StandardMacros.IsValid` _currentfactoryvent
      (:`Is Valid`
        (`/Game/TD/Blueprints/BP_FactoryVent.Interact` _currentfactoryvent)
        (`KismetSystemLibrary.PrintString` "interacted")))))

(event `EnhancedInput|/Game/TD/Input/Actions/IA_SwapCharacters`
  (params (ActionValue :type Boolean) (ElapsedSeconds :type "Float (double-precision)") (TriggeredSeconds :type "Float (double-precision)") (InputAction :type "InputAction Object Reference" :default "/Game/TD/Input/Actions/IA_SwapCharacters.IA_SwapCharacters"))
  (bind _currentplayerpet (`self.CurrentPlayerPet`))
  ; Swap between main character and pet
  (:`Started`
    (`/Engine/EditorBlueprintResources/StandardMacros.IsValid` _currentplayerpet
      (:`Is Valid`
        (`Controller.Possess` (`GameplayStatics.GetPlayerController` 0) _currentplayerpet)
        (`KismetSystemLibrary.PrintString` "pet possessed"))
      (:`Is Not Valid`
        (`KismetSystemLibrary.PrintString` "no valid pet")))))

(event `EnhancedInput|/Game/TD/Input/Actions/IA_Movement`
  (params (ActionValue :type "Vector2D Structure") (ElapsedSeconds :type "Float (double-precision)") (TriggeredSeconds :type "Float (double-precision)") (InputAction :type "InputAction Object Reference" :default "/Game/TD/Input/Actions/IA_Movement.IA_Movement"))
  (bind (_x _y) (`KismetMathLibrary.BreakVector2D` ActionValue))
  (bind (_forward _right) (`self.GetMoveDir`))
  ; Player Movement
  (:`Triggered`
    (`self.AddMovementInput` _forward (* _x (`self.MovementSpeed`)))
    (`self.AddMovementInput` _right (* _y (`self.MovementSpeed`)))))

(event `EnhancedInput|/Game/TD/Input/Actions/IA_PrimaryFire`
  (params (ActionValue :type Boolean) (ElapsedSeconds :type "Float (double-precision)") (TriggeredSeconds :type "Float (double-precision)") (InputAction :type "InputAction Object Reference" :default "/Game/TD/Input/Actions/IA_PrimaryFire.IA_PrimaryFire"))
  ; PrimaryFire
  (:`Started`
    (if (not (`self.IsInBuildingMode`))
      (bind _returnvalue (`|SpawnActorFromClass` "/Game/TD/Blueprints/Projectiles/BP_Projectile.BP_Projectile_C" (`SceneComponent.K2_GetComponentToWorld` (`self.BulletSpawnPoint`)) "Undefined" "MultiplyWithRoot" null null))
      (`/Game/TD/Blueprints/Projectiles/BP_Projectile.DamageUpdate` _returnvalue (`self.AttackDamage`)))))

(event `EnhancedInput|/Game/TD/Input/Actions/IA_FirstPlayerSkill`
  (params (ActionValue :type Boolean) (ElapsedSeconds :type "Float (double-precision)") (TriggeredSeconds :type "Float (double-precision)") (InputAction :type "InputAction Object Reference" :default "/Game/TD/Input/Actions/IA_FirstPlayerSkill.IA_FirstPlayerSkill"))
  ; First Skill
  (:`Started`
    (if (`self.IsInBuildingMode`)
      ;; leave building mode
      (set `self.IsInBuildingMode` false)
      (elif (`self.CanUseFirstSkill`)
        (set `self.CanUseFirstSkill` false)
        (bind _returnvalue (`|SpawnActorFromClass` "/Game/TD/Blueprints/Projectiles/BP_Grenade.BP_Grenade_C" (`SceneComponent.K2_GetComponentToWorld` (`self.BulletSpawnPoint`)) "Undefined" "MultiplyWithRoot" null null))
        (`/Game/TD/Blueprints/Projectiles/BP_Grenade.DamageUpdate` _returnvalue (`self.Power`))
        (`PrimitiveComponent.AddImpulse` (`/Game/TD/Blueprints/Projectiles/BP_Grenade.ProjectileMesh` _returnvalue) (* (`self.GetActorForwardVector` (`GameplayStatics.GetPlayerController` 0)) (1000.0 1000.0 1000.0)) "None" false)
        (`Timeline|FirstSkillCoolDown Timeline` :!via `PlayFromStart`
          (:`Finished`
            (set `self.CanUseFirstSkill` true)))))))

(event `self.ReceiveAnyDamage`
  (params (Damage :type "Float (single-precision)") (DamageType :type "DamageType Object Reference") (InstigatedBy :type "Controller Object Reference") (DamageCauser :type "Actor Object Reference"))
  ; Damage Taken
  (`self.LoseHP` Damage))

(fn `Die`
  (bind _asbp_player_pet (cast `/Game/TD/Blueprints/Player/BP_PlayerPet` self)
    (:`then`
      (`Controller.Possess` (`GameplayStatics.GetPlayerController` 0) (`/Game/TD/Blueprints/Player/BP_PlayerPet.PlayerCharacter` _asbp_player_pet))
      (`self.K2_DestroyActor` _asbp_player_pet))
    (:`CastFailed`
      (`KismetSystemLibrary.PrintString` "YOU DIED"))))

(fn `DragSelectResult`
  (params (SelectedActors :type "Array of Actor Object Reference (by ref)"))
  (returns (NewParam :type Boolean))
  (return false))

(fn `GetLookAtLocation`
  (returns (LookAtLocation :type "Vector Structure"))
  (return (`.Location` (`GameplayStatics.BreakHitResult` (`PlayerController.GetHitResultUnderCursorByChannel` (`GameplayStatics.GetPlayerController` 0) "TraceTypeQuery1" true)))))

(fn `GetMoveDir`
  (returns (Forward :type "Vector Structure") (Right :type "Vector Structure"))
  (bind _camera (`self.Camera`))
  (return (`KismetMathLibrary.Normal` (* (`SceneComponent.GetForwardVector` _camera) (1.0 1.0 0.0))) (`KismetMathLibrary.Normal` (* (`SceneComponent.GetRightVector` _camera) (1.0 1.0 0.0)))))

(fn `LoseHP`
  (params (Damage :type "Float (double-precision)"))
  (bind _output_get (set `self.CurrentHealth` (`KismetMathLibrary.FClamp` (- (`self.CurrentHealth`) Damage) 0.0 (`self.MaxHealth`))))
  (if (<= _output_get 0.0)
    (`self.Die`)))

(fn `PassSelectedUnits`
  (returns (Actors :type "Array of Actor Object Reference"))
  (return))

(fn `UserConstructionScript`)