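; BP_Pet is a pet that follows its owning player and can attack with projectiles.
; BeginPlay sizes the MaxRange sphere from Range, and Tick issues an AI move toward OwningPlayer every frame, a step marked as heavy.
; Attack spawns a BP_Projectile and sets its damage to Power, though nothing here calls it.
; CastSkill and MoveToPlayer are empty stubs.
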(event `self.ReceiveBeginPlay`
  (`SphereComponent.SetSphereRadius` (`self.MaxRange`) (`self.Range`) true))

(event `self.ReceiveTick`
  (params (DeltaSeconds :type "Float (single-precision)"))
  ; Heavy
  (`|AIMoveTo` null (0.0 0.0 0.0) (`self.OwningPlayer`)))

(fn `Attack`
  (returns (HasShot :type Boolean))
  (bind _returnvalue (`|SpawnActorFromClass` "/Game/TD/Blueprints/Projectiles/BP_Projectile.BP_Projectile_C" (`KismetMathLibrary.MakeTransform` (0.0 0.0 0.0)) "Undefined" "MultiplyWithRoot" null null))
  (set `/Game/TD/Blueprints/Projectiles/BP_Projectile.Damage` (`self.Power`) _returnvalue)
  (return false))

(fn `CastSkill`
  ; Skill logic
)

(fn `MoveToPlayer`)

(fn `UserConstructionScript`)