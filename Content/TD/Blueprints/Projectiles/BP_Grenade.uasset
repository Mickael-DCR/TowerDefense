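; Grenade projectile that explodes on a fixed timer started at BeginPlay, with no impact logic in its graph.
; When the delay ends, it spawns a particle effect attached to the mesh and applies radial damage there using its Damage and Radius variables.
; It then destroys only the mesh component, not the actor.
; The Speed variable sets the projectile movement's initial and max speed when that component activates.
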(event `self.ReceiveBeginPlay`
  (bind _projectilemesh (`self.ProjectileMesh`))
  (`KismetSystemLibrary.Delay` 5.0)
  (`GameplayStatics.SpawnEmitterAttached` "/Engine/Tutorial/SubEditors/TutorialAssets/TutorialParticleSystem.TutorialParticleSystem" _projectilemesh)
  (`GameplayStatics.ApplyRadialDamage` :`BaseDamage` (`self.Damage`) :`Origin` (`SceneComponent.K2_GetComponentLocation` _projectilemesh) :`DamageRadius` (`self.Radius`) :`DamageCauser` null :`InstigatedByController` null)
  (`ActorComponent.K2_DestroyComponent` (`self.ProjectileMesh`)))

(event `self.ProjectileMovement.OnComponentActivated`
  (params (Component :type "ActorComponent Object Reference") (bReset :type Boolean))
  (bind _projectilemovement (`self.ProjectileMovement`))
  (bind _speed (`self.Speed`))
  ; Set the Bullet's velocity
  (set `ProjectileMovementComponent.MaxSpeed` _speed _projectilemovement)
  (set `ProjectileMovementComponent.InitialSpeed` _speed _projectilemovement))

(fn `UserConstructionScript`)