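; BP_FactoryInsideVent is the exit vent inside a factory that returns control from the player's pet to the player character.
; When a pet overlaps its box and CanUseDoor is set, it ends the FactoryCore countdown and refunds one available pet to the cached player character, clamped to the maximum.
; It then has the player controller possess the character and destroys the pet; otherwise it prints that the core must be destroyed first.
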(event `self.ReceiveBeginPlay`
  (bind _returnvalue (`GameplayStatics.GetActorOfClass` "/Game/TD/Blueprints/Player/BP_PlayerCharacter.BP_PlayerCharacter_C"))
  (set `self.Player Character` _returnvalue))

(event `self.Box.OnComponentBeginOverlap`
  (params (OverlappedComponent :type "PrimitiveComponent Object Reference") (OtherActor :type "Actor Object Reference") (OtherComp :type "PrimitiveComponent Object Reference") (OtherBodyIndex :type Integer) (bFromSweep :type Boolean) (SweepResult :type "HitResult Structure (by ref)"))
  (bind _player_character (`self.Player Character`))
  ; Send Info to player character
  (bind _asbp_player_pet (cast `/Game/TD/Blueprints/Player/BP_PlayerPet` OtherActor))
  (bind _output_get (set `self.PlayerPet` _asbp_player_pet))
  (if (`/Game/TD/Blueprints/Player/BP_PlayerPet.CanUseDoor` _output_get)
    (`/Game/TD/Blueprints/BP_FactoryCore.EndCountdown` (`self.FactoryCore`))
    (set `/Game/TD/Blueprints/Player/BP_PlayerCharacter.NumberOfPetsAvailable` (`KismetMathLibrary.Clamp` (+ (`/Game/TD/Blueprints/Player/BP_PlayerCharacter.NumberOfPetsAvailable` _player_character) 1) 0 (`/Game/TD/Blueprints/Player/BP_PlayerCharacter.MaxNumberOfPetsAvailable` _player_character)) _player_character)
    (`Controller.Possess` (`GameplayStatics.GetPlayerController` 0) (`self.Player Character`))
    (`self.K2_DestroyActor` (`self.PlayerPet`))
    (else
      (`KismetSystemLibrary.PrintString` "You need to destroy the factory's core before leaving !"))))

(fn `UserConstructionScript`)